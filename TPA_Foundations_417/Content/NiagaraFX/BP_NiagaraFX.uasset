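; Reusable Blueprint wrapper around a Niagara component that plays an effect on demand and reports when it ends.
; PlayFX activates the component with a reset, so each call restarts the system from the beginning.
; When the system finishes, it broadcasts OnFXFinished, then sets the component inactive rather than destroying anything.
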(event `self.NiagaraFX.OnSystemFinished`
  (params (PSystem :type "NiagaraComponent Object Reference"))
  (`self.OnFXFinished` self)
  (`ActorComponent.SetActive` (`self.NiagaraFX`) false false))

(fn `PlayFX`
  (`ActorComponent.SetActive` (`self.NiagaraFX`) true true))

(fn `UserConstructionScript`)