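; Niagara effect spawner that fires on a looping timer, with optional actor pooling.
; Without pooling, each tick spawns and activates an effect at a random spawn point.
; With pooling, pre-spawned actors are activated without being moved, and finish events return in-use actors to the pool after a reset.
; Checkout reads index 0 again after removal, so the in-use list records the next pooled actor instead of the activated one.
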(event `self.ReceiveBeginPlay`
  (if (`self.usePooling`)
    (`self.InitializePoolingSystem`))
  (`KismetSystemLibrary.K2_SetTimerDelegate` (delegate `OnFXSpawnTimerFired`) (`self.FXSpawnDelay`) true))

(event `OnFXSpawnTimerFired`
  (if (`self.usePooling`)
    (`KismetSystemLibrary.PrintString` (`KismetStringLibrary.Conv_IntToString` (`KismetArrayLibrary.Array_Length` (`self.BP_NiagaraFXPool`))))
    (`self.GetRandomSpawnTransform`)
    (bind _wassuccessfullyused (`self.TryUseAvailableFX`))
    (if (not _wassuccessfullyused)
      (`KismetSystemLibrary.PrintString` "Not enough Niagara FX in pool. Try increasing Niagara FX size"))
    (else
      (bind _newparam (`self.GetRandomSpawnTransform`))
      (bind _returnvalue (`|SpawnActorFromClass` (`self.BP_NiagaraFX`) _newparam "Undefined" "MultiplyWithRoot" null null))
      (`self.ActivateNiagaraFX` _returnvalue))))

(fn `ActivateNiagaraFX`
  (params (BP_NiagaraFX :type "/Game/NiagaraFX/BP_NiagaraFX Object Reference"))
  (`ActorComponent.Activate` (`/Game/NiagaraFX/BP_NiagaraFX.NiagaraFX` BP_NiagaraFX) false))

(fn `GetRandomSpawnTransform`
  (returns (NewParam :type "Transform Structure"))
  (return (`self.GetTransform` (`|GetArrayItem` (`self.FXSpawnPoints`) (`KismetMathLibrary.RandomInteger` (`KismetArrayLibrary.Array_Length` (`self.FXSpawnPoints`)))))))

(fn `InitializePoolingSystem`
  (for _ (range 1 (+ (`self.poolSize`) 1))
    (bind _returnvalue (`|SpawnActorFromClass` (`self.BP_NiagaraFX`) (`KismetMathLibrary.MakeTransform` (0.0 0.0 0.0)) "Undefined" "MultiplyWithRoot" null null))
    (`KismetArrayLibrary.Array_Add` (`self.BP_NiagaraFXPool`) _returnvalue)
    (add `/Game/NiagaraFX/BP_NiagaraFX.OnFXFinished` _returnvalue (`|CreateDelegate` :!event `OnNiagaraFXFinished`))))

(fn `OnNiagaraFXFinished`
  (params (BP_NiagaraFX :type "/Game/NiagaraFX/BP_NiagaraFX Object Reference"))
  (bind _niagarafx (`/Game/NiagaraFX/BP_NiagaraFX.NiagaraFX` BP_NiagaraFX))
  (if (`KismetArrayLibrary.Array_Contains` (`self.NiagaFXInUse`) BP_NiagaraFX)
    (`KismetArrayLibrary.Array_RemoveItem` (`self.NiagaFXInUse`) BP_NiagaraFX)
    (`KismetArrayLibrary.Array_Add` (`self.BP_NiagaraFXPool`) BP_NiagaraFX)
    (`ActorComponent.Deactivate` _niagarafx)
    (`NiagaraComponent.ResetSystem` _niagarafx)
    (else
      (`KismetSystemLibrary.PrintString` "Triggered Niagara FX Finished, but it wasn't found to be in use."))))

(fn `TryUseAvailableFX`
  (returns (WasSuccessfullyUsed :type Boolean))
  (bind _bp_niagarafxpool (`self.BP_NiagaraFXPool`))
  (bind _returnvalue (`KismetArrayLibrary.Array_IsEmpty` _bp_niagarafxpool))
  (bind _output (`|GetArrayItem` _bp_niagarafxpool))
  (if (not _returnvalue)
    (`self.ActivateNiagaraFX` _output)
    (`KismetArrayLibrary.Array_RemoveItem` _bp_niagarafxpool _output)
    (`KismetArrayLibrary.Array_Add` (`self.NiagaFXInUse`) _output))
  (return (not _returnvalue)))

(fn `UserConstructionScript`)